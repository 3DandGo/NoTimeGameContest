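; BP_Cart is a cart actor that lets the sloth boy player start or stop using it with the R key.
; It caches the player character on BeginPlay, and its Box overlap with that character's CartInteractionBlock enables input and opens a gate.
; Inside range, R toggles StartCart or StopCart based on IsUsingCart; leaving disables input and closes the gate.
; Its BPI_Interact implementation only prints a debug message and returns false.
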(event OnComponentBeginOverlap(Box)
  (params (OverlappedComponent :type Primitive%20Component%20Object%20Reference) (OtherActor :type Actor%20Object%20Reference) (OtherComp :type Primitive%20Component%20Object%20Reference) (OtherBodyIndex :type Integer) (bFromSweep :type Boolean) (SweepResult :type Hit%20Result%20Structure%20%28by%20ref%29))
  (bind _as_bp_sloth_boy (Variables|Default|GetAs%20BP%20Sloth%20Boy))
  (bind _as_bp_sloth_boy_2 (Variables|Default|GetAs%20BP%20Sloth%20Boy)
    (:then
      (if (== OtherComp (Variables|/Game/Blueprints/SlothBoy/BP_SlothBoy.BP_SlothBoy_C|GetCartInteractionBlock _as_bp_sloth_boy_2))
        (Development|PrintString "In Range To Interact With Cart" true true "(R=0.050727,G=1.000000,B=0.000000,A=1.000000)")
        (Input|EnableInput (Game|GetPlayerController 0))
        (Utilities|FlowControl|Gate true) ; enters at Open
      ))
    (:else)))

(event OnComponentEndOverlap(Box)
  (params (OverlappedComponent :type Primitive%20Component%20Object%20Reference) (OtherActor :type Actor%20Object%20Reference) (OtherComp :type Primitive%20Component%20Object%20Reference) (OtherBodyIndex :type Integer))
  (bind _as_bp_sloth_boy (Variables|Default|GetAs%20BP%20Sloth%20Boy))
  (bind _as_bp_sloth_boy_2 (Variables|Default|GetAs%20BP%20Sloth%20Boy)
    (:then
      (if (== OtherComp (Variables|/Game/Blueprints/SlothBoy/BP_SlothBoy.BP_SlothBoy_C|GetCartInteractionBlock _as_bp_sloth_boy_2))
        (Development|PrintString "Out Of Range" true true "(R=1.000000,G=0.000444,B=0.120198,A=1.000000)")
        (Input|DisableInput (Game|GetPlayerController 0))
        (Utilities|FlowControl|Gate true) ; enters at Close
      ))
    (:else)))

(event EventBeginPlay
  (bind _asbp_sloth_boy (Utilities|Casting|CastToBP_SlothBoy (Game|GetPlayerCharacter 0)))
  (Variables|Default|SetAs%20BP%20Sloth%20Boy _asbp_sloth_boy))

(event Collision|EventActorBeginOverlap
  (params (OtherActor :type Actor%20Object%20Reference)))

(event EventTick
  (params (DeltaSeconds :type Float%20%28single-precision%29)))

(event Input|KeyboardEvents|R
  (params (Key :type Key%20Structure :default "None"))
  (bind _as_bp_sloth_boy (Variables|Default|GetAs%20BP%20Sloth%20Boy))
  (:Pressed
    (Utilities|FlowControl|Gate true
      (:Exit
        (Development|PrintString "The Gate Is Open" true true "(R=1.000000,G=0.724685,B=0.000000,A=1.000000)")
        (if (Variables|/Game/Blueprints/SlothBoy/BP_SlothBoy.BP_SlothBoy_C|GetbIsUsingCart (Variables|Default|GetAs%20BP%20Sloth%20Boy))
          (Default|StopCart _as_bp_sloth_boy)
          (else
            (Default|StartCart _as_bp_sloth_boy)))))))

(fn ConstructionScript)

(fn BPIInteract
  (Development|PrintString "Interaction Called" true true "(R=1.000000,G=0.684446,B=0.000000,A=1.000000)")
  (return false))