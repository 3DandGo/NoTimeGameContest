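; BP_SlothBoy is the player-controlled sloth character, with first- and third-person cameras.
; BeginPlay adds an Enhanced Input mapping context for jumping, camera-relative movement, looking, and dashing, which raises walk speed while held.
; The Q key toggles between the two cameras by activating one and deactivating the other.
; CartInteractionBlock overlaps with a BP_Cart's Box send that cart an interaction message after a BPI_Interactions check on the component.
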(event OnComponentBeginOverlap(CartInteractionBlock)
  (params (OverlappedComponent :type Primitive%20Component%20Object%20Reference) (OtherActor :type Actor%20Object%20Reference) (OtherComp :type Primitive%20Component%20Object%20Reference) (OtherBodyIndex :type Integer) (bFromSweep :type Boolean) (SweepResult :type Hit%20Result%20Structure%20%28by%20ref%29))
  (bind _asbp_cart (Utilities|Casting|CastToBP_Cart OtherActor))
  (if (== OtherComp (Variables|/Game/Blueprints/Cart/BP_Cart.BP_Cart_C|GetBox _asbp_cart))
    (if (Utilities|DoesObjectImplementInterface OtherComp "/Game/Blueprints/Interfaces/BPI_Interactions.BPI_Interactions_C")
      (Class|BPIInteractions|BPIInteract(Message) _asbp_cart))))

(event OnComponentEndOverlap(CartInteractionBlock)
  (params (OverlappedComponent :type Primitive%20Component%20Object%20Reference) (OtherActor :type Actor%20Object%20Reference) (OtherComp :type Primitive%20Component%20Object%20Reference) (OtherBodyIndex :type Integer)))

(event Input|EnhancedActionEvents|EnhancedInputActionIA_SlothDashing
  (params (ActionValue :type Vector%202D%20Structure) (ElapsedSeconds :type Float%20%28double-precision%29) (TriggeredSeconds :type Float%20%28double-precision%29) (InputAction :type Input%20Action%20Object%20Reference :default "/Game/Blueprints/SlothBoy/Inputs/IA_SlothDashing.IA_SlothDashing"))
  (bind _charactermovement (Variables|Character|GetCharacterMovement))
  (:Started
    (Variables|/Script/Engine.CharacterMovementComponent|SetMaxWalkSpeed _charactermovement 9e+02))
  (:Completed
    (Variables|/Script/Engine.CharacterMovementComponent|SetMaxWalkSpeed _charactermovement 4e+02)))

(event Input|EnhancedActionEvents|EnhancedInputActionIA_SlothJumping
  (params (ActionValue :type Boolean) (ElapsedSeconds :type Float%20%28double-precision%29) (TriggeredSeconds :type Float%20%28double-precision%29) (InputAction :type Input%20Action%20Object%20Reference :default "/Game/Blueprints/SlothBoy/Inputs/IA_SlothJumping.IA_SlothJumping"))
  (:Started
    (Character|Jump))
  (:Completed
    (Character|StopJumping)))

(event Input|EnhancedActionEvents|EnhancedInputActionIA_SlothMoving
  (params (ActionValue :type Vector%202D%20Structure) (ElapsedSeconds :type Float%20%28double-precision%29) (TriggeredSeconds :type Float%20%28double-precision%29) (InputAction :type Input%20Action%20Object%20Reference :default "/Game/Blueprints/SlothBoy/Inputs/IA_SlothMoving.IA_SlothMoving"))
  (bind _returnvalue (Pawn|GetControlRotation :!class /Script/Engine.Pawn))
  (Pawn|Input|AddMovementInput (Math|Vector|GetRightVector (Math|Rotator|MakeRotator (.roll _returnvalue) 0.0 (.yaw _returnvalue))) (.x ActionValue) false)
  (Pawn|Input|AddMovementInput (Math|Vector|GetForwardVector (Math|Rotator|MakeRotator 0.0 0.0 (.yaw (Pawn|GetControlRotation :!class /Script/Engine.Pawn)))) (.y ActionValue) false))

(event Input|EnhancedActionEvents|EnhancedInputActionIA_SlothLooking
  (params (ActionValue :type Vector%202D%20Structure) (ElapsedSeconds :type Float%20%28double-precision%29) (TriggeredSeconds :type Float%20%28double-precision%29) (InputAction :type Input%20Action%20Object%20Reference :default "/Game/Blueprints/SlothBoy/Inputs/IA_SlothLooking.IA_SlothLooking"))
  (Pawn|Input|AddControllerYawInput (.x ActionValue))
  (Pawn|Input|AddControllerPitchInput (.y ActionValue)))

(event Input|EnhancedActionEvents|EnhancedInputActionIA_SlothInteract
  (params (ActionValue :type Boolean) (ElapsedSeconds :type Float%20%28double-precision%29) (TriggeredSeconds :type Float%20%28double-precision%29) (InputAction :type Input%20Action%20Object%20Reference :default "/Game/Blueprints/SlothBoy/Inputs/IA_SlothInteract.IA_SlothInteract")))

(event EventBeginPlay
  (Input|AddMappingContext (PlayerController|LocalPlayerSubsystems|GetEnhancedInputLocalPlayerSubsystem (Game|GetPlayerController 0)) "/Game/Blueprints/SlothBoy/Inputs/IA_SlothDefaultMapping.IA_SlothDefaultMapping" 0 "(bIgnoreAllPressedKeysUntilRelease=True,bForceImmediately=False,bNotifyUserSettings=False)"))

(event Collision|EventActorBeginOverlap
  (params (OtherActor :type Actor%20Object%20Reference)))

(event EventTick
  (params (DeltaSeconds :type Float%20%28single-precision%29)))

(event Input|KeyboardEvents|Q
  (params (Key :type Key%20Structure :default "None"))
  (:Pressed
    (if (Variables|Default|GetbThirdPersonCameraInUse)
      (Components|Activation|Activate (Variables|Default|GetFirstPersonCamera) false)
      (Components|Activation|Deactivate (Variables|Default|GetThirdPersonCamera))
      (Variables|Default|SetbThirdPersonCameraInUse false)
      (else
        (Components|Activation|Activate (Variables|Default|GetThirdPersonCamera) false)
        (Components|Activation|Deactivate (Variables|Default|GetFirstPersonCamera))
        (Variables|Default|SetbThirdPersonCameraInUse true)))))

(fn ConstructionScript)